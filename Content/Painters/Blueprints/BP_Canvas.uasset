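; BP_Canvas is a paintable surface actor that accumulates brush strokes in render targets.
; On BeginPlay it creates color and mask render targets sized from mesh scale and feeds them to a dynamic M_Canvas material on the mesh.
; DrawBrush stamps a brush texture at a normalized location into both targets, using colored and white brush materials.
; Tick randomizes the paint color every frame, so strokes vary in color.
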(event `self.ReceiveBeginPlay`
  (bind _returnvalue (* 1 100))
  (bind (_x _y) (`KismetMathLibrary.BreakVector3f` (`SceneComponent.K2_GetComponentScale` (`self.StaticMesh`))))
  (bind _returnvalue_2 (`KismetMathLibrary.FTrunc` (* _x _returnvalue)))
  (bind _returnvalue_3 (`KismetMathLibrary.FTrunc` (* _y _returnvalue)))
  (`|ExecutionSequence`
    (:`then_0`
      (bind _returnvalue_4 (`KismetRenderingLibrary.CreateRenderTarget2D` _returnvalue_2 _returnvalue_3))
      (bind _output_get (set `self.RenderTarget` _returnvalue_4))
      (`KismetRenderingLibrary.ClearRenderTarget2D` _output_get (struct)))
    (:`then_1`
      (bind _returnvalue_5 (`KismetRenderingLibrary.CreateRenderTarget2D` _returnvalue_2 _returnvalue_3))
      (bind _output_get_2 (set `self.RenderTargetMask` _returnvalue_5))
      (`KismetRenderingLibrary.ClearRenderTarget2D` _output_get_2 (struct)))
    (:`then_2`
      (bind _returnvalue_6 (`KismetMaterialLibrary.CreateDynamicMaterialInstance` "/Game/Painters/Materials/M_Canvas.M_Canvas"))
      (`MaterialInstanceDynamic.SetTextureParameterValue` _returnvalue_6 "RenderTarget" (`self.RenderTarget`))
      (`MaterialInstanceDynamic.SetTextureParameterValue` _returnvalue_6 "RenderTargetMask" (`self.RenderTargetMask`))
      (`PrimitiveComponent.SetMaterial` (`self.StaticMesh`) 0 _returnvalue_6))
    (:`then_3`
      (bind _returnvalue_7 (`KismetMaterialLibrary.CreateDynamicMaterialInstance` "/Game/Painters/Materials/M_Brush.M_Brush"))
      (set `self.BrushMaterial` _returnvalue_7))
    (:`then_4`
      (bind _returnvalue_8 (`KismetMaterialLibrary.CreateDynamicMaterialInstance` "/Game/Painters/Materials/M_WhiteBrush.M_WhiteBrush"))
      (set `self.WhtieBrushMaterial` _returnvalue_8))))

(event `self.ReceiveTick`
  (params (DeltaSeconds :type "Float (single-precision)"))
  (`MaterialInstanceDynamic.SetVectorParameterValue` (`self.BrushMaterial`) "PaintColor" (`KismetMathLibrary.MakeColor` (`KismetMathLibrary.RandomFloatInRange` 0.0 1.0) (`KismetMathLibrary.RandomFloatInRange` 0.0 1.0) (`KismetMathLibrary.RandomFloatInRange` 0.0 1.0))))

(fn `DrawBrush`
  (params (BrushTexture :type "Texture2D Object Reference") (BrushSize :type "Float (double-precision)") (DrawLocation :type "Vector2D Structure"))
  (bind _returnvalue (* BrushSize 1.0))
  (`|ExecutionSequence`
    (:`then_0`
      (`MaterialInstanceDynamic.SetTextureParameterValue` (`self.BrushMaterial`) "BrushTexture" BrushTexture)
      (`MaterialInstanceDynamic.SetTextureParameterValue` (`self.WhtieBrushMaterial`) "WhiteBrushTexture" BrushTexture))
    (:`then_1`
      (bind (_canvas _size _context) (`KismetRenderingLibrary.BeginDrawCanvasToRenderTarget` (`self.RenderTarget`)))
      (`Canvas.K2_DrawMaterial` _canvas (`self.BrushMaterial`) (`KismetMathLibrary.Conv_VectorToVector2D` (- (* _size DrawLocation) (/ _returnvalue 2.0))) (`KismetMathLibrary.MakeVector2D` _returnvalue _returnvalue) (0.0 0.0) (1.0 1.0) 0.0 (0.5 0.5))
      (`KismetRenderingLibrary.EndDrawCanvasToRenderTarget` _context))
    (:`then_2`
      (bind (_canvas_2 _size_2 _context_2) (`KismetRenderingLibrary.BeginDrawCanvasToRenderTarget` (`self.RenderTargetMask`)))
      (`Canvas.K2_DrawMaterial` _canvas_2 (`self.WhtieBrushMaterial`) (`KismetMathLibrary.Conv_VectorToVector2D` (- (* _size_2 DrawLocation) (/ _returnvalue 2.0))) (`KismetMathLibrary.MakeVector2D` _returnvalue _returnvalue) (0.0 0.0) (1.0 1.0) 0.0 (0.5 0.5))
      (`KismetRenderingLibrary.EndDrawCanvasToRenderTarget` _context_2))))

(fn `UserConstructionScript`)